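; Player-controlled rocket pawn that maps Enhanced Input to thrust, staging and look controls.
; Traction and reduce inputs add or decrease power on BPRocketSceneComponent, the stage-reset input advances it to the next step, and look drives controller yaw and inverted pitch.
; The component is initialized in the construction script, and BPI camera and pivot getters return the current step's socket location so the view follows the active stage.
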(event Input|EnhancedActionEvents|EnhancedInputActionIA_AddTraction
  (params (ActionValue :type Float%20%28double-precision%29) (ElapsedSeconds :type Float%20%28double-precision%29) (TriggeredSeconds :type Float%20%28double-precision%29) (InputAction :type Input%20Action%20Object%20Reference :default "/Game/Input/InputAction/IA_AddTraction.IA_AddTraction"))
  (:Triggered
    (Default|AddPower (Variables|Default|GetBP_RocketSceneComponent) ActionValue :!label _label))
  (:Completed
    (goto _label)))

(event Input|EnhancedActionEvents|EnhancedInputActionIA_ReduceCravings
  (params (ActionValue :type Float%20%28double-precision%29) (ElapsedSeconds :type Float%20%28double-precision%29) (TriggeredSeconds :type Float%20%28double-precision%29) (InputAction :type Input%20Action%20Object%20Reference :default "/Game/Input/InputAction/IA_ReduceCravings.IA_ReduceCravings"))
  (:Triggered
    (Default|DecreasePower (Variables|Default|GetBP_RocketSceneComponent) ActionValue :!label _label))
  (:Completed
    (goto _label)))

(event Input|EnhancedActionEvents|EnhancedInputActionIA_ResetStage
  (params (ActionValue :type Boolean) (ElapsedSeconds :type Float%20%28double-precision%29) (TriggeredSeconds :type Float%20%28double-precision%29) (InputAction :type Input%20Action%20Object%20Reference :default "/Game/Input/InputAction/IA_ResetStage.IA_ResetStage"))
  (:Started
    (Default|NextStep (Variables|Default|GetBP_RocketSceneComponent))))

(event Input|EnhancedActionEvents|EnhancedInputActionIA_Look
  (params (ActionValue :type Vector%202D%20Structure) (ElapsedSeconds :type Float%20%28double-precision%29) (TriggeredSeconds :type Float%20%28double-precision%29) (InputAction :type Input%20Action%20Object%20Reference :default "/Game/Input/InputAction/IA_Look.IA_Look"))
  (bind (_x _y) (Math|Vector2D|BreakVector2D ActionValue))
  (:Triggered
    (Pawn|Input|AddControllerYawInput _x :!label _label)
    (Pawn|Input|AddControllerPitchInput (* _y -1.0)))
  (:Completed
    (goto _label)))

(fn ConstructionScript
  (Default|Initialize (Variables|Default|GetBP_RocketSceneComponent) self))

(fn GetRocketSceneComponent
  (return (Variables|Default|GetBP_RocketSceneComponent)))

(fn BPIGetCameraTarget
  (return (Default|FindCurrentStepSocketLocation (Variables|Default|GetBP_RocketSceneComponent))))

(fn BPIGetPivotTarget
  (return (Math|Transform|MakeTransform (Default|FindCurrentStepSocketLocation (Variables|Default|GetBP_RocketSceneComponent)))))