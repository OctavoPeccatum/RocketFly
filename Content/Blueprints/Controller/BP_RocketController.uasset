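; Player controller for the rocket that sets up input and drives the rocket HUD.
; On BeginPlay it adds the Enhanced Input mapping context, creates WBP_RocketUI and caches the scene component from the controlled BP_Rocket.
; Tick pushes distance as height, current step and power to the UI, while a looping timer refreshes the current step's fuel mass less often.
; On possession it forwards the pawn to BP_RocketCameraManager.
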(event Custom|Fuel
  (Default|UpdateFuel (Variables|Default|GetUI) (Variables|/Game/Blueprints/Components/BP_RocketStaticMeshComponent.BP_RocketStaticMeshComponent_C|GetCurrentFuelMass (Variables|/Game/Blueprints/Components/BP_RocketSceneComponent.BP_RocketSceneComponent_C|GetCurrentComponentStep (Variables|Default|GetBP%20Rocket%20Scene%20Component)))))

(event EventBeginPlay
  (Input|AddMappingContext (PlayerController|LocalPlayerSubsystems|GetEnhancedInputLocalPlayerSubsystem) "/Game/Input/IMC_Defaults.IMC_Defaults" 0 "(bIgnoreAllPressedKeysUntilRelease=True,bForceImmediately=False)")
  (bind _returnvalue (UserInterface|CreateWidget "/Game/UI/WBP_RocketUI.WBP_RocketUI_C" self))
  (bind _output_get (Variables|Default|SetUI _returnvalue))
  (UserInterface|Viewport|AddtoViewport _output_get 0)
  (bind _asbp_rocket (Utilities|Casting|CastToBP_Rocket (Pawn|GetControlledPawn)))
  (bind _bp_rocketscenecomponent (Default|GetRocketSceneComponent _asbp_rocket))
  (Variables|Default|SetBP%20Rocket%20Scene%20Component _bp_rocketscenecomponent)
  (Utilities|Time|SetTimerbyEvent (delegate Custom|Fuel) 0.2 true))

(event EventTick
  (params (DeltaSeconds :type Float%20%28single-precision%29))
  (bind _bp_rocket_scene_component (Variables|Default|GetBP%20Rocket%20Scene%20Component))
  (Default|UpdateHeight (Variables|Default|GetUI) (Variables|/Game/Blueprints/Components/BP_RocketSceneComponent.BP_RocketSceneComponent_C|GetDistance _bp_rocket_scene_component))
  (Default|UpdateStep (Variables|Default|GetUI) (Variables|/Game/Blueprints/Components/BP_RocketSceneComponent.BP_RocketSceneComponent_C|GetCurrentStep _bp_rocket_scene_component))
  (Default|UpdatePower (Variables|Default|GetUI) (Variables|/Game/Blueprints/Components/BP_RocketSceneComponent.BP_RocketSceneComponent_C|GetPower _bp_rocket_scene_component)))

(event EventPossess
  (params (PossessedPawn :type Pawn%20Object%20Reference))
  (bind _asbp_rocket_camera_manager (Utilities|Casting|CastToBP_RocketCameraManager (Variables|Default|GetPlayerCameraManager)))
  (Default|OnPossess _asbp_rocket_camera_manager PossessedPawn))

(fn ConstructionScript)