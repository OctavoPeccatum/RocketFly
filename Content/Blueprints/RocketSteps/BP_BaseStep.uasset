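; BP_BaseStep is a base Blueprint for a rocket step, holding a mesh and its fuel mass.
; BeginPlay sets the current fuel mass to the starting value, and DecreaseFuel subtracts a given mass flow from it, with no clamping.
; GetMesh returns the step's static mesh along with the result of looking up its "Docking" socket.
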(event EventBeginPlay
  (Variables|Default|SetCurrentFuelMass (Variables|Default|GetStartFuelMass)))

(event Collision|EventActorBeginOverlap
  (params (OtherActor :type Actor%20Object%20Reference)))

(event EventTick
  (params (DeltaSeconds :type Float%20%28single-precision%29)))

(fn ConstructionScript)

(fn GetMesh
  (bind _staticmesh (Variables|Default|GetStaticMesh))
  (bind _staticmesh_2 (Variables|/Script/Engine.StaticMeshComponent|GetStaticMesh _staticmesh))
  (return _staticmesh_2 (Class|StaticMesh|FindSocket _staticmesh_2 "Docking")))

(fn DecreaseFuel
  (params (MassFlow :type Float%20%28double-precision%29))
  (Variables|Default|SetCurrentFuelMass (- (Variables|Default|GetCurrentFuelMass) MassFlow)))