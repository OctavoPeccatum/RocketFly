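; Player camera manager that takes over the camera with a fixed wide FOV for view targets tagged "Rocket", deferring to the parent for others.
; It follows an offset pivot from the possessed pawn's interface, lagging it per axis in camera-yaw space at one shared speed.
; Rotation eases toward control rotation, and small directional offsets place the camera.
; On possess, it passes controller and pawn to the ABP_PlayerCameraBehavior anim instance.
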(event Custom|OnPossess
  (params (NewPawn :type Pawn%20Object%20Reference))
  (Variables|Default|SetControlledPawn NewPawn)
  (bind _asabp_player_camera_behavior (Utilities|Casting|CastToABP_PlayerCameraBehavior (Components|SkeletalMesh|GetAnimInstance (Variables|Default|GetCameraBehavior))))
  (Variables|/Game/Blueprints/CameraSystem/ABP_PlayerCameraBehavior.ABP_PlayerCameraBehavior_C|SetPlayerController _asabp_player_camera_behavior (Game|Player|GetOwningPlayerController))
  (Variables|/Game/Blueprints/CameraSystem/ABP_PlayerCameraBehavior.ABP_PlayerCameraBehavior_C|SetControlledPawn _asabp_player_camera_behavior (Variables|Default|GetControlledPawn)))

(fn ConstructionScript)

(fn BlueprintUpdateCamera
  (params (CameraTarget :type Actor%20Object%20Reference))
  (if (Actor|ActorHasTag CameraTarget "Rocket")
    (bind (_location _rotation) (CallFunction|CustomCameraBehavior))
    (return _location _rotation 1.2e+02 true)
    (else
      (bind (_newcameralocation _newcamerarotation _newcamerafov _returnvalue) (|CallParentFunction CameraTarget))
      (return _newcameralocation _newcamerarotation _newcamerafov _returnvalue))))

(fn CustomCameraBehavior
  (Utilities|FlowControl|Sequence
    (:then_0
      (bind _transform (Class|BPICamera|BPIGetPivotTarget(Message) (Variables|Default|GetControlledPawn)))
      (Variables|Default|SetPivotTarget (Math|Transform|MakeTransform (+ (.Location (Math|Transform|BreakTransform _transform)) "1000.000000,0.000000,10.000000") (.Rotation (Math|Transform|BreakTransform _transform)) (.Scale (Math|Transform|BreakTransform _transform)))))
    (:then_1
      (Variables|Default|SetTargetCameraRotation (Math|Interpolation|RInterpTo (Camera|GetCameraRotation) (Pawn|GetControlRotation (Game|Player|GetOwningPlayerController) :!class /Script/Engine.Controller) (Utilities|Time|GetWorldDeltaSeconds) 0.5)))
    (:then_2
      (Variables|Default|SetSmoothedPivotTarget (Math|Transform|MakeTransform (CallFunction|CalculateAxisIndependentLag (.location (Variables|Default|GetSmoothedPivotTarget)) (.location (Variables|Default|GetPivotTarget)) (Variables|Default|GetTargetCameraRotation)) (.rotation (Variables|Default|GetPivotTarget)))))
    (:then_3
      (Variables|Default|SetPivotLocation (+ (.location (Variables|Default|GetSmoothedPivotTarget)) (* (Math|Vector|GetForwardVector (.rotation (Variables|Default|GetSmoothedPivotTarget))) 1.0) (* (Math|Vector|GetRightVector (.rotation (Variables|Default|GetSmoothedPivotTarget))) 1.0) (* (Math|Vector|GetUpVector (.rotation (Variables|Default|GetSmoothedPivotTarget))) 1.0))))
    (:then_4
      (Variables|Default|SetTargetCameraLocation (+ (Variables|Default|GetPivotLocation) (* (Math|Vector|GetForwardVector (Variables|Default|GetTargetCameraRotation)) 0.5) (* (Math|Vector|GetRightVector (Variables|Default|GetTargetCameraRotation)) 0.5) (* (Math|Vector|GetUpVector (Variables|Default|GetTargetCameraRotation)) 0.5))))
    (:then_5
      (return (.Location (Math|Transform|BreakTransform (Math|Transform|MakeTransform (Variables|Default|GetTargetCameraLocation) (Variables|Default|GetTargetCameraRotation)))) (.Rotation (Math|Transform|BreakTransform (Math|Transform|MakeTransform (Variables|Default|GetTargetCameraLocation) (Variables|Default|GetTargetCameraRotation))))))))

(fn CalculateAxisIndependentLag
  (params (CurrentLocation :type Vector) (TargetLocation :type Vector) (CameraRotation :type Rotator))
  (bind _returnvalue (Utilities|Time|GetWorldDeltaSeconds))
  (bind _interp_speed (Variables|Default|GetInterp%20Speed))
  (LocalVariables|SetCameraRotationYaw (Math|Rotator|MakeRotator 0.0 0.0 (.yaw CameraRotation)))
  (return (Math|Vector|RotateVector (Math|Vector|MakeVector (Math|Interpolation|FInterpTo (.x (Math|Vector|UnrotateVector CurrentLocation (LocalVariables|GetCameraRotationYaw))) (.x (Math|Vector|UnrotateVector TargetLocation (LocalVariables|GetCameraRotationYaw))) _returnvalue _interp_speed) (Math|Interpolation|FInterpTo (.y (Math|Vector|UnrotateVector CurrentLocation (LocalVariables|GetCameraRotationYaw))) (.y (Math|Vector|UnrotateVector TargetLocation (LocalVariables|GetCameraRotationYaw))) _returnvalue _interp_speed) (Math|Interpolation|FInterpTo (.z (Math|Vector|UnrotateVector CurrentLocation (LocalVariables|GetCameraRotationYaw))) (.z (Math|Vector|UnrotateVector TargetLocation (LocalVariables|GetCameraRotationYaw))) _returnvalue _interp_speed)) (LocalVariables|GetCameraRotationYaw))))