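; Rocket component that builds a multi-stage rocket on its Actor and moves it along local up while power and current-stage fuel remain.
; BeginPlay stacks stage mesh components via "Docking" sockets, then reverses the list so the first-spawned stage burns first.
; Each tick, speed follows a Tsiolkovsky-style log mass ratio scaled by power, and a curve sets fuel burn.
; NextStep detaches the active stage with physics and cuts power to roughly a third.
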(event EventBeginPlay
  (bind _components (Variables|Default|GetComponents))
  (CallFunction|SpawnSteps)
  (Utilities|Array|Reverse _components)
  (Variables|Default|SetCurrentComponentStep (Utilities|Array|Get(acopy) _components (Utilities|Array|LastIndex _components))))

(event EventTick
  (params (DeltaSeconds :type Float%20%28single-precision%29))
  (if (and (> (Variables|Default|GetPower) 0.0) (> (Variables|/Game/Blueprints/Components/BP_RocketStaticMeshComponent.BP_RocketStaticMeshComponent_C|GetCurrentFuelMass (Variables|Default|GetCurrentComponentStep)) 0.0))
    (Transformation|AddActorLocalOffset (Variables|Default|GetActor) (* "0.000000,0.000000,1.000000" (CallFunction|TakeoffSpeed)) true false)
    (Default|DecreaseFuel (Variables|Default|GetCurrentComponentStep) (CallFunction|GetMassFlow))))

(fn AddPower
  (params (ActionValue :type Float%20%28double-precision%29))
  (if (<= (+ (Variables|Default|GetPower) ActionValue) 1e+02)
    (Variables|Default|SetPower (+ (Variables|Default|GetPower) ActionValue))))

(fn DecreasePower
  (params (ActionValue :type Float%20%28double-precision%29))
  (if (>= (- (Variables|Default|GetPower) ActionValue) 0.0)
    (Variables|Default|SetPower (- (Variables|Default|GetPower) ActionValue))))

(fn SpawnSteps
  (for (_array_element _array_index) (Variables|Default|GetStepArray)
    (if (== _array_index 0)
      (CallFunction|SpawnStaticMesh :NewMesh (.stepmesh _array_element) :StartFuelMass (.fuelmass _array_element) :CapsuleWeight (.capsulemass _array_element))
      (else
        (bind _output_get (LocalVariables|SetVector (+ (LocalVariables|GetVector) (Variables|/Script/Engine.StaticMeshSocket|GetRelativeLocation (Class|StaticMesh|FindSocket (Variables|/Script/Engine.StaticMeshComponent|GetStaticMesh (Utilities|Array|Get(acopy) (Variables|Default|GetComponents) (- _array_index 1))) "Docking")))))
        (CallFunction|SpawnStaticMesh (.stepmesh _array_element) (Math|Transform|MakeTransform _output_get "0, 0, 0" "1.000000,1.000000,1.000000") (.fuelmass _array_element) (.capsulemass _array_element))))))

(fn TakeoffSpeed
  (bind _capsuleweight (CallFunction|GetCapsuleWeight))
  (return (* (Variables|Default|GetPower) (Math|Float|Loge (/ (+ (Variables|/Game/Blueprints/Components/BP_RocketStaticMeshComponent.BP_RocketStaticMeshComponent_C|GetCurrentFuelMass (Variables|Default|GetCurrentComponentStep)) _capsuleweight) _capsuleweight)))))

(fn GetMassFlow
  (return (Math|Curves|GetFloatValue (Variables|Default|GetMassFlowToTime) (Variables|Default|GetPower))))

(fn GetCapsuleWeight
  (for _array_element (Variables|Default|GetComponents)
    (LocalVariables|SetWeight (+ (LocalVariables|GetWeight) (Variables|/Game/Blueprints/Components/BP_RocketStaticMeshComponent.BP_RocketStaticMeshComponent_C|GetCurrentFuelMass _array_element) (Variables|/Game/Blueprints/Components/BP_RocketStaticMeshComponent.BP_RocketStaticMeshComponent_C|GetCapsuleWeight _array_element))))
  (return (LocalVariables|GetWeight)))

(fn Initialize
  (params (Actor :type Actor%20Object%20Reference))
  (Variables|Default|SetActor Actor))

(fn SpawnStaticMesh
  (params (NewMesh :type Static%20Mesh%20Object%20Reference) (RelativeTransform :type Transform) (StartFuelMass :type Float%20%28double-precision%29) (CapsuleWeight :type Float%20%28double-precision%29))
  (bind _returnvalue (Game|AddComponentbyClass (Variables|Default|GetActor) "/Game/Blueprints/Components/BP_RocketStaticMeshComponent.BP_RocketStaticMeshComponent_C" false RelativeTransform StartFuelMass CapsuleWeight))
  (Components|StaticMesh|SetStaticMesh _returnvalue NewMesh)
  (Utilities|Array|Add (Variables|Default|GetComponents) _returnvalue)
  (return _returnvalue))

(fn FindCurrentStepSocketLocation
  (bind _components (Variables|Default|GetComponents))
  (return (Transformation|GetSocketLocation (Utilities|Array|Get(acopy) _components (Utilities|Array|LastIndex _components)) "Docking")))

(fn NextStep
  (bind _components (Variables|Default|GetComponents))
  (if (> (Utilities|Array|Length (Variables|Default|GetComponents)) 1)
    (Physics|SetSimulatePhysics (Variables|Default|GetCurrentComponentStep) true)
    (Transformation|DetachFromComponent (Variables|Default|GetCurrentComponentStep) "KeepWorld" "KeepWorld" "KeepWorld" true)
    (Utilities|Array|Resize _components (- (Utilities|Array|Length _components) 1))
    (Variables|Default|SetCurrentComponentStep (Utilities|Array|Get(acopy) _components (Utilities|Array|LastIndex _components)))
    (Math|Integer|IncrementInt (Variables|Default|GetCurrentStep)
      (:%20%20
        (Variables|Default|SetPower (Math|Conversions|ToFloat(Integer) (Math|Float|Ceil (/ (Variables|Default|GetPower) 3.0))))))))